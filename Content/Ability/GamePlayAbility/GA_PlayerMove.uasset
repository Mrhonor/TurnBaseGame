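; GA_PlayerMove is a gameplay ability that executes a move order for a turn-based character on the grid.
; On activation it checks that the current order is a move, feeds its target location into grid movement input, and ends when movement completes or is interrupted.
; On end it updates the grid manager, clears the executing flag, and broadcasts order completion for player shadow characters.
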(event Ability|EventActivateAbility
  (bind _asturn_base_character (Utilities|Casting|CastToTurnBaseCharacter (Ability|GetOwningActorfromActorInfo))
    (:then
      (if (Utilities|Enum|Equal(Enum) (.ordertype (Class|OrderProcessComponent|GetCurrentExecuteOrder (Class|TurnBaseCharacter|GetOrderProcessComponent _asturn_base_character))) "EMoveOrder")
        (|AddGridMovementInput _asturn_base_character (.targetlocation (Class|OrderProcessComponent|GetCurrentExecuteOrder (Class|TurnBaseCharacter|GetOrderProcessComponent _asturn_base_character)))
          (:OnComplete
            _)
          (:OnInterrupted
            _))
        (Ability|EndAbility)
        (else
          (Ability|EndAbility))))
    (:CastFailed
      (Ability|EndAbility))))

(event Ability|EventOnEndAbility
  (params (bWasCancelled :type Boolean))
  (bind _asturn_base_character (Utilities|Casting|CastToTurnBaseCharacter (Ability|GetOwningActorfromActorInfo)))
  (Class|GridManagerComponent|UpdateGrid (Variables|/Script/TurnBaseGame.OrderProcessComponent|GetCurrentGridManager (Class|TurnBaseCharacter|GetOrderProcessComponent _asturn_base_character)) _asturn_base_character (.currentlocation (Class|OrderProcessComponent|GetCurrentExecuteOrder (Class|TurnBaseCharacter|GetOrderProcessComponent _asturn_base_character))))
  (Class|OrderProcessComponent|SetOrderExecuting (Class|TurnBaseCharacter|GetOrderProcessComponent _asturn_base_character) false)
  (bind _asbp_turn_base_player_character_shadow (Utilities|Casting|CastToBP_TurnBasePlayerCharacterShadow _asturn_base_character))
  (Default|BroadcastOrderFinish _asbp_turn_base_player_character_shadow (Class|OrderProcessComponent|GetCurrentExecuteOrder (Class|TurnBaseCharacter|GetOrderProcessComponent _asturn_base_character))))