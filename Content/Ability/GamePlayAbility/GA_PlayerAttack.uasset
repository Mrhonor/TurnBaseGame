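; GA_PlayerAttack is a Gameplay Ability that performs the player's attack.
; On activation it plays the attack montage on the owning Character's mesh and ends the ability when the montage completes, blends out or is interrupted.
; When the ability ends, it clears the executing flag on the owner's OrderProcessComponent, if one exists.
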(event Ability|EventActivateAbility
  (Development|PrintString "AttackAbility")
  (bind _ascharacter (Utilities|Casting|CastToCharacter (Ability|GetOwningActorfromActorInfo)))
  (Animation|Montage|PlayMontage (Variables|/Script/Engine.Character|GetMesh _ascharacter) "/Game/Blueprint/Character/Player/Anim/PlayerAttackMontage.PlayerAttackMontage"
    (:OnCompleted
      _)
    (:OnBlendOut
      _)
    (:OnInterrupted
      _))
  (Ability|EndAbility))

(event Ability|EventOnEndAbility
  (params (bWasCancelled :type Boolean))
  (bind _returnvalue (Ability|GetOwningActorfromActorInfo))
  (bind _returnvalue_2 (Actor|GetComponentbyClass _returnvalue "/Script/TurnBaseGame.OrderProcessComponent"))
  (Utilities|IsValid _returnvalue_2
    (:Is%20Valid
      (Class|OrderProcessComponent|SetOrderExecuting _returnvalue_2 false))))