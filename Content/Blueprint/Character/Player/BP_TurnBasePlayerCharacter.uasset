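; Turn-based player character Blueprint that turns input into attack orders during the Battle Prepare state.
; Holding A arms the attack state, and a left click then queues an attack order from the shadow actor's location toward the mouse location.
; The order goes to both the character's and the shadow actor's OrderProcessComponent, but only the shadow is told to execute its first order immediately.
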(event EventBeginPlay)

(event Collision|EventActorBeginOverlap
  (params (OtherActor :type Actor%20Object%20Reference)))

(event EventKeyPressed
  (params (key :type Key%20Structure :default "None"))
  (bind _shadowplayercomponent (Variables|Default|GetShadowPlayerComponent))
  (bind _shadowplayercomponent_2 (Variables|Default|GetShadowPlayerComponent))
  (bind _playerinputmessage (Variables|Default|GetPlayerInputMessage))
  (bind _mouselocation (Utilities|Struct|BreakPlayerCameraInput _playerinputmessage))
  (bind _returnvalue (Class|ShadowPlayerComponent|GetShadowActor _shadowplayercomponent))
  (bind _returnvalue_2 (Class|ShadowPlayerComponent|GetShadowActor _shadowplayercomponent_2))
  (bind _returnvalue_3 (Transformation|GetActorLocation _returnvalue))
  (bind _returnvalue_4 (Class|TurnBaseCharacter|GetOrderProcessComponent _returnvalue_2))
  (bind _orderinput (Utilities|Struct|MakeOrderInput "EAttackOrder" _mouselocation _returnvalue_3 "(GameplayTags=((TagName=\"Order.Attack\")))"))
  (Variables|Default|SetKeyValue key)
  (switch Utilities|FlowControl|Switch|SwitchonETurnBasePlayState (Variables|Default|GetCurrentGameState)
    (:EBattlePrepare
      (if (Variables|Default|GetAttackState)
        (if (and (Class|OrderProcessComponent|CanAddOrderInput (Variables|Default|GetOrderProcessComponent)) (== (Variables|Default|GetKeyValue) "LeftMouseButton"))
          (Class|OrderProcessComponent|AddOrderInput (Variables|Default|GetOrderProcessComponent) _orderinput)
          (Class|OrderProcessComponent|AddOrderInput _returnvalue_4 _orderinput)
          (Class|OrderProcessComponent|ExecuteFirstOrder _returnvalue_4)
          (Development|PrintString "Exe"))
        (else
          (Variables|Default|SetAttackState (== (Variables|Default|GetKeyValue) "A")))))))

(event EventKeyReleased
  (params (key :type Key%20Structure :default "None"))
  (Variables|Default|SetKeyValue key)
  (switch Utilities|FlowControl|Switch|SwitchonETurnBasePlayState (Variables|Default|GetCurrentGameState)
    (:EBattlePrepare
      (if (== (Variables|Default|GetKeyValue) "A")
        (Variables|Default|SetAttackState false)))))

(fn ConstructionScript)