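; Order-processing component for a turn-based character that executes the first queued order on its owner.
; ExecuteFirstOrder branches on order type: Move feeds the target location into the TurnBaseCharacter as grid movement input, while Attack activates Gameplay Abilities by the order's tag.
; Both mark an order as executing, then remove it from the list; unknown orders are simply removed.
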(event EventBeginPlay)

(event EventTick
  (params (DeltaSeconds :type Float%20%28single-precision%29)))

(event EventExecuteFirstOrder
  (bind _returnvalue (Class|OrderProcessComponent|GetFirstOrder))
  (bind _returnvalue_2 (Components|GetOwner))
  (Variables|Default|SetOrder _returnvalue)
  (switch Utilities|FlowControl|Switch|SwitchonEOrderType (.OrderType (Utilities|Struct|BreakOrderInput _returnvalue))
    (:EMoveOrder
      (bind _asturn_base_character (Utilities|Casting|CastToTurnBaseCharacter _returnvalue_2))
      (Class|TurnBaseCharacter|AddGridMovementInput _asturn_base_character (.targetlocation (Variables|Default|GetOrder)))
      (Class|OrderProcessComponent|SetOrderExecuting true :!label _label))
    (:EAttackOrder
      (Abilities|TryActivateAbilitiesbyTag (Ability|GetAbilitySystemComponent _returnvalue_2) (GameplayTags|MakeGameplayTagContainerfromTag "(TagName=\"Order.Attack\")") true)
      (goto _label))
    (:EUnknowOrder
      _))
  (Utilities|Array|RemoveIndex (Variables|Default|GetOrderList)))